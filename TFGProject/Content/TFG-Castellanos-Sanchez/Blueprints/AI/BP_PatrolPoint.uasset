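; AI patrol point actor that links to others through NextPoint and PreviusPoint arrays, returning a random neighbour forwards or backwards.
; DrawSplines visualizes each outgoing link with a hidden spline lined with instanced arrows, using the both-direction arrow when the target lists this point in PreviusPoint.
; The construction script redraws this point and its neighbours, while UpdateAllSpline redraws every patrol point.
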(fn `DrawSplines`
  (locals (CurrentPoint :type "/Game/TFG-Castellanos-Sanchez/Blueprints/AI/BP_PatrolPoint Object Reference") (CurrentSpline :type "SplineComponent Object Reference") (SelectedDirectionArrow :type "InstancedStaticMeshComponent Object Reference"))
  (for _array_element (`self.K2_GetComponentsByClass` "/Script/Engine.SplineComponent")
    (`ActorComponent.K2_DestroyComponent` _array_element))
  (`InstancedStaticMeshComponent.ClearInstances` (`self.BothDirectionArrow`))
  (`InstancedStaticMeshComponent.ClearInstances` (`self.SingleDirectionArrow`))
  (for _array_element_2 (`self.NextPoint`)
    (set `local.CurrentPoint` _array_element_2)
    (bind _returnvalue (`AddComponent|NODE_AddSplineComponent-0`))
    (bind _output_get (set `local.CurrentSpline` _returnvalue))
    (`SceneComponent.SetVisibility` _output_get false false)
    (`SceneComponent.K2_AttachToComponent` (`local.CurrentSpline`) (`self.Cube`) "None" "SnapToTarget" "KeepRelative" "KeepRelative" true)
    (`SplineComponent.SetLocationAtSplinePoint` (`local.CurrentSpline`) 0 (`SceneComponent.K2_GetComponentLocation` (`self.Cube`)) "World" false)
    (`SplineComponent.SetLocationAtSplinePoint` (`local.CurrentSpline`) 1 (`SceneComponent.K2_GetComponentLocation` (`/Game/TFG-Castellanos-Sanchez/Blueprints/AI/BP_PatrolPoint.Cube` (`local.CurrentPoint`))) "World" true)
    (set `local.SelectedDirectionArrow` (select `bool` (`KismetArrayLibrary.Array_Contains` (`/Game/TFG-Castellanos-Sanchez/Blueprints/AI/BP_PatrolPoint.PreviusPoint` (`local.CurrentPoint`)) self) :`false` (`self.SingleDirectionArrow`) :`true` (`self.BothDirectionArrow`)))
    (for _index (range 1 (+ (`KismetMathLibrary.FFloor` (/ (`SplineComponent.GetSplineLength` (`local.CurrentSpline`)) 50.0)) 1))
      (bind _meshlocation (`self.GetLocationAtIndex` (`local.CurrentSpline`) _index 15.0))
      (`InstancedStaticMeshComponent.AddInstance` (`local.SelectedDirectionArrow`) (`KismetMathLibrary.MakeTransform` _meshlocation (`KismetMathLibrary.MakeRotFromX` (- (`self.GetLocationAtIndex` (`local.CurrentSpline`) (+ _index 1) 15.0) _meshlocation)) (0.5 0.5 0.5)) false))))

(fn `GetLocationAtIndex`
  (params (CurrentSpline :type "SplineComponent Object Reference") (Index :type Integer) (Spacing :type "Float (double-precision)"))
  (returns (MeshLocation :type "Vector Structure"))
  (return (`SplineComponent.GetLocationAtDistanceAlongSpline` CurrentSpline (* Index Spacing) "Local")))

(fn `GetNextPatrolPoints`
  (params (InForwards :type Boolean))
  (returns (PatrolPoint :type "/Game/TFG-Castellanos-Sanchez/Blueprints/AI/BP_PatrolPoint Object Reference"))
  (return (`KismetArrayLibrary.Array_Random` (select `bool` InForwards :`false` (`self.PreviusPoint`) :`true` (`self.NextPoint`)))))

(fn `UpdateAllSpline`
  (bind _outactors (`GameplayStatics.GetAllActorsOfClass` "BP_PatrolPoint_C"))
  (for _array_element _outactors
    (`self.DrawSplines` _array_element)))

(fn `UserConstructionScript`
  (locals (TotalPoints :type Integer))
  (`self.DrawSplines`)
  (for _array_element (`self.PreviusPoint`)
    (`self.DrawSplines` _array_element))
  (for _array_element_2 (`self.NextPoint`)
    (`self.DrawSplines` _array_element_2)))