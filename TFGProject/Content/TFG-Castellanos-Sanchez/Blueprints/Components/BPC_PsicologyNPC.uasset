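; NPC psychology component that maintains a social memory of nearby actors and feeds social stimuli into an emotion AI (TestEmotioAI).
; A looping timer runs a sphere trace for pawns, assigning the player and "Secondary"-tagged actors roles derived from the GameInstance's player role.
; Clamped, range-mapped distances update the NPC1 and NPC2 inputs, while witnessed attacks pass aggressor and victim roles.
; It also stores an actor to follow, optionally remembering the previous one.
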(event `self.ReceiveBeginPlay`
  (`self.SetBehaviourTick` 0.3))

(event `ServerBehaviourTick`
  (if (`self.CanTakeAction`)
    (`self.SetDistancesNPCs`)
    (`self.CurrentTarget`
      (:`then`)
      (:`else`))))

(event `SetBehaviourTick`
  (params (TickInterval :type "Float (double-precision)"))
  (`KismetSystemLibrary.K2_ClearAndInvalidateTimerHandle` (`self.BehaviourTickTimerHandle`))
  (bind _returnvalue (`KismetSystemLibrary.K2_SetTimerDelegate` (delegate `ServerBehaviourTick`) TickInterval true))
  (set `self.BehaviourTickTimerHandle` _returnvalue))

(event `OnWitneesAttack`
  (params (Agresor :type "Actor Object Reference") (Victima :type "Actor Object Reference"))
  (bind (_value _returnvalue) (`BlueprintMapLibrary.Map_Find` (`self.SocialMemory`) Agresor))
  (bind (_value_2 _returnvalue_2) (`BlueprintMapLibrary.Map_Find` (`self.SocialMemory`) Victima))
  (if _returnvalue
    (set `self.RolAgresor` _value)
    (if _returnvalue_2
      (set `self.RolVictima` _value_2)
      (`self.SetRolesEmotionAI`)
      (elif (== Victima (`self.GetOwner`))
        (set `self.RolVictima` "NewEnumerator1")
        (`self.SetRolesEmotionAI`)))))

(event `/Game/TFG-Castellanos-Sanchez/Blueprints/Interfaces/BI_NPCComponent.SetActorToFollow`
  (params (NewActor :type "Actor Object Reference") (ShouldRememberOldActor :type Boolean))
  (if ShouldRememberOldActor
    (set `self.OldActorToFollow` (`self.ActorToFollow`))
    (set `self.ActorToFollow` NewActor)
    (else
      (set `self.ActorToFollow` NewActor)
      (set `self.OldActorToFollow` null))))

(fn `CalculateDistance`
  (params (Objetivo :type "Actor Object Reference"))
  (returns (Distance :type "Float (double-precision)"))
  (return (`KismetMathLibrary.MapRangeClamped` (`KismetMathLibrary.Vector_Distance` (`Actor.K2_GetActorLocation` (`self.GetOwner`)) (`Actor.K2_GetActorLocation` Objetivo)) 100.0 1000.0 1.0)))

(fn `FindActorInRange`
  (params (Range :type "Float (double-precision)"))
  (locals (CurrentActorInLoop :type "Actor Object Reference"))
  (bind _returnvalue (`Actor.K2_GetActorLocation` (`self.GetOwner`)))
  (bind _outhits (`KismetSystemLibrary.SphereTraceMultiForObjects` _returnvalue _returnvalue Range (`|MakeArray` "ObjectTypeQuery3" :!type "EObjectTypeQuery Enum")))
  (for _array_element _outhits
    (set `local.CurrentActorInLoop` (`.HitActor` (`GameplayStatics.BreakHitResult` _array_element)))
    (if (not (`KismetArrayLibrary.Array_Contains` (`self.AllActorsInRange`) (`local.CurrentActorInLoop`)))
      (`KismetArrayLibrary.Array_Add` (`self.AllActorsInRange`) (`local.CurrentActorInLoop`)))))

(fn `SetDistancesNPCs`
  (locals (OppositeRole1 :type "/Game/TFG-Castellanos-Sanchez/Blueprints/Enums/E_SocialRole Enum" :default "NewEnumerator3") (OppositeRole2 :type "/Game/TFG-Castellanos-Sanchez/Blueprints/Enums/E_SocialRole Enum" :default "NewEnumerator2"))
  (`KismetArrayLibrary.Array_Clear` (`self.AllActorsInRange`))
  (set `self.CurrentTarget` null)
  (`self.FindActorInRange` (`self.Range`))
  (for _array_element (`self.AllActorsInRange`)
    (bind (_value _returnvalue) (`BlueprintMapLibrary.Map_Find` (`self.SocialMemory`) _array_element))
    (if _returnvalue
      (`self.SetVariablesEmotionAI` _array_element _value)
      (elif (== _array_element (`GameplayStatics.GetPlayerPawn` 0))
        (bind _asgi_demo (cast `/Game/TFG-Castellanos-Sanchez/Blueprints/Managers/GI_Demo` (`GameplayStatics.GetGameInstance`)))
        (`BlueprintMapLibrary.Map_Add` (`self.SocialMemory`) _array_element (`/Game/TFG-Castellanos-Sanchez/Blueprints/Managers/GI_Demo.PlayerSocialRole` _asgi_demo))
        (`self.SetVariablesEmotionAI` _array_element _value)
        (elif (`Actor.ActorHasTag` _array_element "Secondary")
          (bind _asgi_demo_2 (cast `/Game/TFG-Castellanos-Sanchez/Blueprints/Managers/GI_Demo` (`GameplayStatics.GetGameInstance`)))
          (`BlueprintMapLibrary.Map_Add` (`self.SocialMemory`) _array_element (select `/Game/TFG-Castellanos-Sanchez/Blueprints/Enums/E_SocialRole` (`/Game/TFG-Castellanos-Sanchez/Blueprints/Managers/GI_Demo.PlayerSocialRole` _asgi_demo_2) :`NewEnumerator0` "NewEnumerator0" :`NewEnumerator1` "NewEnumerator0" :`NewEnumerator2` (`local.OppositeRole1`) :`NewEnumerator3` (`local.OppositeRole2`)))
          (`self.SetVariablesEmotionAI` _array_element _value))))))

(fn `SetRolesEmotionAI`
  (bind _testemotioai (`self.TestEmotioAI`))
  (set `/Game/TFG-Castellanos-Sanchez/IA/Test_EmotionAI.Ejecuta_Golpeo` (`|GetEnumeratorNameAsString` (`self.RolAgresor`)) _testemotioai)
  (set `/Game/TFG-Castellanos-Sanchez/IA/Test_EmotionAI.Recibe_Golpeo` (`|GetEnumeratorNameAsString` (`self.RolVictima`)) _testemotioai))

(fn `SetVariablesEmotionAI`
  (params (Objetivo :type "Actor Object Reference") (Selection :type "/Game/TFG-Castellanos-Sanchez/Blueprints/Enums/E_SocialRole Enum" :default "NewEnumerator0"))
  (bind _distance (`self.CalculateDistance` Objetivo))
  (bind _testemotioai (`self.TestEmotioAI`))
  (switch `/Game/TFG-Castellanos-Sanchez/Blueprints/Enums/E_SocialRole` Selection
    (:`NewEnumerator2`
      (set `/Game/TFG-Castellanos-Sanchez/IA/Test_EmotionAI.NPC1` _distance _testemotioai))
    (:`NewEnumerator3`
      (set `/Game/TFG-Castellanos-Sanchez/IA/Test_EmotionAI.NPC2` _distance _testemotioai))))