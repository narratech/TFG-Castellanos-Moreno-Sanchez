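; Actor component that holds a slot-limited inventory of stackable items as an array of item ID and amount pairs.
; AddToInventory tops up existing stacks, then creates new ones while slots remain, returning success and any remainder.
; Stack limits come from Items_DT; the InventoryFull flag is set when space runs out and never cleared here.
; Tick prints the contents every frame for debugging, and BeginPlay caches the player character.
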(event `self.ReceiveBeginPlay`
  (bind _asbp_demo_shooter_character (cast `/Game/TFG-Castellanos-Sanchez/Blueprints/FirstPerson/BP_DemoShooterCharacter` (`GameplayStatics.GetPlayerCharacter` 0)))
  (set `self.PlayerRef` _asbp_demo_shooter_character))

(event `self.ReceiveTick`
  (params (DeltaSeconds :type "Float (single-precision)"))
  (for _array_element (`self.Content`)
    (`KismetSystemLibrary.PrintString` (`KismetTextLibrary.Conv_TextToString` (`|FormatText` "{NAME} / {AMOUNT}" (break `/Game/TFG-Castellanos-Sanchez/Blueprints/Structures/Inventory_Struct` _array_element) (`.Amount_5_25BCF6EA45F07A2E571416A8F9779631` (break `/Game/TFG-Castellanos-Sanchez/Blueprints/Structures/Inventory_Struct` _array_element)))) true true (struct :`G` 0.66 :`B` 1.0 :`A` 1.0) 0.0)))

(fn `Add_To_Inventory`
  (params (Item_ID :type Name) (Amount :type Integer))
  (returns (Added_All :type Boolean) (Remaining :type Integer))
  (locals (Amount_Remainig :type Integer) (Inventory_Full :type Boolean))
  (`|ExecutionSequence`
    (:`then_0`
      (bind _output_get (set `local.Amount_Remainig` Amount))
      (while (and (> _output_get 0) (not (`local.Inventory_Full`)))
        (bind (_slot_found _index _room_in_stack) (`self.Find_Existing_Slot` (`local.Item_ID`)))
        (if _slot_found
          (bind _returnvalue (`KismetMathLibrary.Clamp` (`local.Amount_Remainig`) 0 _room_in_stack))
          (`self.Add_To_Stack` _index _returnvalue)
          (set `local.Amount_Remainig` (- (`local.Amount_Remainig`) _returnvalue))
          (`KismetSystemLibrary.PrintString` "Add to stack")
          (elif (`self.Inventory_Has_Room`)
            (bind _amount_added (`self.Create_New_Stack` (`local.Item_ID`) (`local.Amount_Remainig`)))
            (set `local.Amount_Remainig` (- (`local.Amount_Remainig`) _amount_added))
            (`KismetSystemLibrary.PrintString` "New_Stack")
            (else
              (set `local.Inventory_Full` true)
              (`KismetSystemLibrary.PrintString` "Inventory Full"))))))
    (:`then_1`
      (return (not (`local.Inventory_Full`)) (`local.Amount_Remainig`)))))

(fn `Add_To_Stack`
  (params (Index :type Integer) (Amount :type Integer))
  (bind (_output_item_id _output_amount) (break `/Game/TFG-Castellanos-Sanchez/Blueprints/Structures/Inventory_Struct` (`|GetArrayItem` (`self.Content`) Index)))
  (`KismetArrayLibrary.Array_Set` (`self.Content`) Index (make `/Game/TFG-Castellanos-Sanchez/Blueprints/Structures/Inventory_Struct` _output_item_id (+ _output_amount Amount))))

(fn `Create_New_Stack`
  (params (Item_ID :type Name) (Amount :type Integer))
  (returns (Amount_Added :type Integer))
  (bind _max_stacksize (`self.Get_Max_StackSize` Item_ID))
  (bind _returnvalue (`KismetMathLibrary.SelectInt` _max_stacksize Amount (> Amount _max_stacksize)))
  (`KismetArrayLibrary.Array_Add` (`self.Content`) (make `/Game/TFG-Castellanos-Sanchez/Blueprints/Structures/Inventory_Struct` Item_ID _returnvalue))
  (return _returnvalue))

(fn `Find_Existing_Slot`
  (params (Item_ID :type Name))
  (returns (Slot_Found :type Boolean) (Index :type Integer) (Room_In_Stack :type Integer))
  (bind _item_id (`local.Item_ID`))
  (bind _max_stacksize (`self.Get_Max_StackSize` _item_id))
  (for (_array_element _array_index) (`self.Content`)
    (if (== (break `/Game/TFG-Castellanos-Sanchez/Blueprints/Structures/Inventory_Struct` _array_element) _item_id)
      (if (< (`.Amount_5_25BCF6EA45F07A2E571416A8F9779631` (break `/Game/TFG-Castellanos-Sanchez/Blueprints/Structures/Inventory_Struct` _array_element)) _max_stacksize)
        (return true _array_index (- _max_stacksize (`.Amount_5_25BCF6EA45F07A2E571416A8F9779631` (break `/Game/TFG-Castellanos-Sanchez/Blueprints/Structures/Inventory_Struct` _array_element))))))))

(fn `Get_Item_Details`
  (params (Item_ID :type Name))
  (returns (Out_Row :type "/Game/TFG-Castellanos-Sanchez/Blueprints/Structures/Item_Struct Structure"))
  (bind _returnvalue (`|GetDataTableRow` "/Game/TFG-Castellanos-Sanchez/Blueprints/Datatables/Items_DT.Items_DT" Item_ID)
    (:`then`
      (return _returnvalue))))

(fn `Get_Max_StackSize`
  (params (Item_ID :type Name))
  (returns (Max_StackSize :type Integer))
  (bind (_out_row_item_id _out_row_icon _out_row_max_stacksize) (break `/Game/TFG-Castellanos-Sanchez/Blueprints/Structures/Item_Struct` (`self.Get_Item_Details` Item_ID)))
  (return _out_row_max_stacksize))

(fn `Inventory_Has_Room`
  (returns (Has_Room :type Boolean))
  (return (< (`KismetArrayLibrary.Array_Length` (`self.Content`)) (`self.Inventory_Size`))))