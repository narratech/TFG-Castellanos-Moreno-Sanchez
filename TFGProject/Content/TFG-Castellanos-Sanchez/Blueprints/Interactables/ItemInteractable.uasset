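; An interactable item pickup that adds its item ID and amount to the player's inventory component.
; On a full add it also passes the hardcoded demo pistol class to the player and destroys itself; otherwise it keeps and prints the remaining amount.
; An overlap volume shows or hides an interaction icon widget for the demo shooter character, and SetFocus forwards focus state to that widget.
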(event `self.ReceiveBeginPlay`
  (`self.BeginPlay_Get_Refs`))

(event `/Game/TFG-Castellanos-Sanchez/Blueprints/Interfaces/Interactable.Interact`
  (params (PlayerRef :type "/Game/TFG-Castellanos-Sanchez/Blueprints/FirstPerson/BP_DemoShooterCharacter Object Reference"))
  (bind (_added_all _remaining) (`/Game/TFG-Castellanos-Sanchez/Blueprints/Components/BPC_Inventory.Add_To_Inventory` (`/Game/TFG-Castellanos-Sanchez/Blueprints/FirstPerson/BP_DemoShooterCharacter.BPC_Inventory` PlayerRef) (`self.Item ID`) (`self.Amount`)))
  (if _added_all
    (message `/Game/TFG-Castellanos-Sanchez/Blueprints/Weapons/BPI_WeaponHolderDemo.Add Weapon Class` PlayerRef "/Game/TFG-Castellanos-Sanchez/Blueprints/Weapons/BP_ShooterWeapon_PistolDemo.BP_ShooterWeapon_PistolDemo_C")
    (`self.K2_DestroyActor`)
    (else
      (bind _output_get (set `self.Amount` _remaining))
      (`KismetSystemLibrary.PrintString` (`KismetStringLibrary.Conv_IntToString` _output_get)))))

(event `self.Interaction_Icon_Show_Collision.OnComponentBeginOverlap`
  (params (OverlappedComponent :type "PrimitiveComponent Object Reference") (OtherActor :type "Actor Object Reference") (OtherComp :type "PrimitiveComponent Object Reference") (OtherBodyIndex :type Integer) (bFromSweep :type Boolean) (SweepResult :type "HitResult Structure (by ref)"))
  (cast `/Game/TFG-Castellanos-Sanchez/Blueprints/FirstPerson/BP_DemoShooterCharacter` OtherActor)
  (`/Game/TFG-Castellanos-Sanchez/Blueprints/HUD/W_Interaction_Icon.Show/Hide` (`self.Interact_Ico_Widget_ref`) true))

(event `self.Interaction_Icon_Show_Collision.OnComponentEndOverlap`
  (params (OverlappedComponent :type "PrimitiveComponent Object Reference") (OtherActor :type "Actor Object Reference") (OtherComp :type "PrimitiveComponent Object Reference") (OtherBodyIndex :type Integer))
  (cast `/Game/TFG-Castellanos-Sanchez/Blueprints/FirstPerson/BP_DemoShooterCharacter` OtherActor)
  (`/Game/TFG-Castellanos-Sanchez/Blueprints/HUD/W_Interaction_Icon.Show/Hide` (`self.Interact_Ico_Widget_ref`) false))

(event `self.Set_Focus`
  (params (Focus :type Boolean))
  (`/Game/TFG-Castellanos-Sanchez/Blueprints/HUD/W_Interaction_Icon.Set_Focus` (`self.Interact_Ico_Widget_ref`) Focus))

(fn `BeginPlay_Get_Refs`
  (bind _asw_interaction_icon (cast `/Game/TFG-Castellanos-Sanchez/Blueprints/HUD/W_Interaction_Icon` (`WidgetComponent.GetWidget` (`self.Interact_Icon`))))
  (set `self.Interact_Ico_Widget_ref` _asw_interaction_icon))

(fn `Get_Details`
  (returns (Result :type Boolean))
  (return true))

(fn `UserConstructionScript`)