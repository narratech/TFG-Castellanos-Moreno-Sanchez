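; Drives personality- and emotion-based facial and body animation for a MetaHuman character.
; Weighted, clamped sums of four MBTI-style axes (IE, NS, TS, JP) set expression, facial dynamics and posture targets; WeightT multiplies JP and WeightJ TS.
; BeginPlay installs a post-process AnimBP on the MetaHuman's head mesh.
; Tick pushes interpolated face settings, posture and the emotion struct to face and body AnimInstances through Blueprint interfaces.
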(event `self.ReceiveTick`
  (params (DeltaSeconds :type "Float (single-precision)"))
  ;[0.8281 0.7723 0 0.9043] Update
  (`self.Event_TickFacial` DeltaSeconds)
  (`self.Event_TickCorporal` DeltaSeconds))

(event `self.ReceiveEndPlay`
  (params (EndPlayReason :type "EEndPlayReason Enum" :default "Destroyed"))
  ;[0 0.4041 0.5156] Ended
  (`self.Reset`))

(event `self.ReceiveBeginPlay`
  ; Setup
  (`self.Event_BeginFacial`))

(event `/Game/TFG-Castellanos-Sanchez/Blueprints/Interfaces/BPI_EmotionIA.SetEmotions`
  (params (Emociones :type "Map of String to Float (double-precision)"))
  (`self.UpdateEmotionsStruct` Emociones))

(event `/Game/TFG-Castellanos-Sanchez/Blueprints/Interfaces/BPI_EmotionIA.SetPersonality`
  (params (`I/E` :type "Float (double-precision)") (`N/S` :type "Float (double-precision)") (`T/S` :type "Float (double-precision)") (`J/P` :type "Float (double-precision)"))
  (set `self.I/E` `I/E`)
  (set `self.N/S` `N/S`)
  (set `self.T/S` `T/S`)
  (set `self.J/P` `J/P`)
  (`self.Event_SetSetupFacial`)
  (`self.Event_SetSetupCorporal`))

(event `Event_TickCorporal`
  (params (Time :type "Float (double-precision)"))
  (`self.UpdateCorporal` Time))

(event `Event_SetSetupCorporal`
  ; Setup
  (bind _personality (`self.CalculateRawCorporalTargets`))
  (bind _output_get (set `self.AuxCorporalPersonalitySettings` _personality))
  (bind _transfer (`self.TransferCorporalSettigns` _output_get))
  (set `self.CorporalPersonalitySettings` _transfer))

(event `Event_TickFacial`
  (params (Time :type "Float (double-precision)"))
  ;[0.8281 0.7723 0 0.9043] Update
  (set `self.IsTicking` true)
  (`self.Update` Time))

(event `Event_BeginFacial`
  ; Setup
  (bind _metahumanactor (`self.MetahumanActor`)
    (:`then`
      (bind _asdemo_sandbox_character_mover (cast `/Game/TFG-Castellanos-Sanchez/Blueprints/NPCs/DemoSandboxCharacter_Mover` _metahumanactor))
      (bind _output_get (set `self.Metahuman` (`ChildActorComponent.ChildActor` (`/Game/TFG-Castellanos-Sanchez/Blueprints/NPCs/DemoSandboxCharacter_Mover.VisualOverride` _asdemo_sandbox_character_mover))))
      (`self.Find Face` _output_get))
    (:`else`)))

(event `Event_SetSetupFacial`
  (`self.SetupFacial`))

(fn `Apply_Emotion_To_Struct`
  (params (value :type "Float (double-precision)") (Selection :type String))
  (locals (valueEmotion :type "Float (double-precision)"))
  (set `local.valueEmotion` value)
  (switch `string` Selection
    (:`Ira`
      (setmembers `/Game/TFG-Castellanos-Sanchez/Blueprints/Settings/ST_IAEmotions` :`StructRef` (`self.IAEmotionsSettings`) :`Angry` (`local.value`)))
    (:`Molesto`
      (setmembers `/Game/TFG-Castellanos-Sanchez/Blueprints/Settings/ST_IAEmotions` :`StructRef` (`self.IAEmotionsSettings`) :`Annoyed` (`local.value`)))
    (:`Aburrimiento`
      (setmembers `/Game/TFG-Castellanos-Sanchez/Blueprints/Settings/ST_IAEmotions` :`StructRef` (`self.IAEmotionsSettings`) :`Bored` (`local.value`)))
    (:`Infantil`
      (setmembers `/Game/TFG-Castellanos-Sanchez/Blueprints/Settings/ST_IAEmotions` :`StructRef` (`self.IAEmotionsSettings`) :`Childish` (`local.value`)))
    (:`Confuso`
      (setmembers `/Game/TFG-Castellanos-Sanchez/Blueprints/Settings/ST_IAEmotions` :`StructRef` (`self.IAEmotionsSettings`) :`Confused` (`local.value`)))
    (:`Curioso`
      (setmembers `/Game/TFG-Castellanos-Sanchez/Blueprints/Settings/ST_IAEmotions` :`StructRef` (`self.IAEmotionsSettings`) :`Curious` (`local.value`)))
    (:`Disgusto`
      (setmembers `/Game/TFG-Castellanos-Sanchez/Blueprints/Settings/ST_IAEmotions` :`StructRef` (`self.IAEmotionsSettings`) :`Disguted` (`local.value`)))
    (:`Verguenza`
      (setmembers `/Game/TFG-Castellanos-Sanchez/Blueprints/Settings/ST_IAEmotions` :`StructRef` (`self.IAEmotionsSettings`) :`Embarrased` (`local.value`)))
    (:`Emocionado`
      (setmembers `/Game/TFG-Castellanos-Sanchez/Blueprints/Settings/ST_IAEmotions` :`StructRef` (`self.IAEmotionsSettings`) :`Excited` (`local.value`)))
    (:`Miedo`
      (setmembers `/Game/TFG-Castellanos-Sanchez/Blueprints/Settings/ST_IAEmotions` :`StructRef` (`self.IAEmotionsSettings`) :`Fearful` (`local.value`)))
    (:`Concentracion`
      (setmembers `/Game/TFG-Castellanos-Sanchez/Blueprints/Settings/ST_IAEmotions` :`StructRef` (`self.IAEmotionsSettings`) :`Focused` (`local.value`)))
    (:`Felicidad`
      (setmembers `/Game/TFG-Castellanos-Sanchez/Blueprints/Settings/ST_IAEmotions` :`StructRef` (`self.IAEmotionsSettings`) :`Happy` (`local.value`)))
    (:`Enamorado`
      (setmembers `/Game/TFG-Castellanos-Sanchez/Blueprints/Settings/ST_IAEmotions` :`StructRef` (`self.IAEmotionsSettings`) :`Love` (`local.value`)))
    (:`Nervioso`
      (setmembers `/Game/TFG-Castellanos-Sanchez/Blueprints/Settings/ST_IAEmotions` :`StructRef` (`self.IAEmotionsSettings`) :`Nervous` (`local.value`)))
    (:`Dolor`
      (setmembers `/Game/TFG-Castellanos-Sanchez/Blueprints/Settings/ST_IAEmotions` :`StructRef` (`self.IAEmotionsSettings`) :`Pained` (`local.value`)))
    (:`Orgullo`
      (setmembers `/Game/TFG-Castellanos-Sanchez/Blueprints/Settings/ST_IAEmotions` :`StructRef` (`self.IAEmotionsSettings`) :`Proud` (`local.value`)))
    (:`Relajado`
      (setmembers `/Game/TFG-Castellanos-Sanchez/Blueprints/Settings/ST_IAEmotions` :`StructRef` (`self.IAEmotionsSettings`) :`Relaxed` (`local.value`)))
    (:`Tristeza`
      (setmembers `/Game/TFG-Castellanos-Sanchez/Blueprints/Settings/ST_IAEmotions` :`StructRef` (`self.IAEmotionsSettings`) :`Sad` (`local.value`)))
    (:`Sorpresa`
      (setmembers `/Game/TFG-Castellanos-Sanchez/Blueprints/Settings/ST_IAEmotions` :`StructRef` (`self.IAEmotionsSettings`) :`Surprised` (`local.value`)))
    (:`Sospechoso`
      (setmembers `/Game/TFG-Castellanos-Sanchez/Blueprints/Settings/ST_IAEmotions` :`StructRef` (`self.IAEmotionsSettings`) :`Suspicious` (`local.value`)))
    (:`Cansancio`
      (setmembers `/Game/TFG-Castellanos-Sanchez/Blueprints/Settings/ST_IAEmotions` :`StructRef` (`self.IAEmotionsSettings`) :`Tired` (`local.value`)))))

(fn `Calculate_Corporal_Canal`
  (params (Weight_E :type "Float (double-precision)") (Weight_N :type "Float (double-precision)") (Weight_T :type "Float (double-precision)") (Weight_J :type "Float (double-precision)") (Base_Offset :type "Float (double-precision)") (MinAngle :type "Float (double-precision)") (Max_Angle :type "Float (double-precision)"))
  (returns (resul_Value :type "Float (double-precision)"))
  (return (`KismetMathLibrary.Lerp` MinAngle Max_Angle (`KismetMathLibrary.FClamp` (+ (+ (+ (+ Base_Offset (* (`self.I/E`) Weight_E)) (* (`self.N/S`) Weight_N)) (* (`self.J/P`) Weight_T)) (* (`self.T/S`) Weight_J))))))

(fn `Calculate_Single_Curve`
  (params (Weight_E :type "Float (double-precision)") (Weight_N :type "Float (double-precision)") (Weight_T :type "Float (double-precision)") (Weight_J :type "Float (double-precision)") (Base_Offset :type "Float (double-precision)"))
  (returns (resul_Value :type "Float (double-precision)"))
  (return (`KismetMathLibrary.FClamp` (+ (+ (+ (+ Base_Offset (* (`self.I/E`) Weight_E)) (* (`self.N/S`) Weight_N)) (* (`self.J/P`) Weight_T)) (* (`self.T/S`) Weight_J)) -1.0)))

(fn `Calculate_Single_CurveWithRange`
  (params (Weight_E :type "Float (double-precision)") (Weight_N :type "Float (double-precision)") (Weight_T :type "Float (double-precision)") (Weight_J :type "Float (double-precision)") (Base_Offset :type "Float (double-precision)") (Min :type "Float (double-precision)") (Max :type "Float (double-precision)"))
  (returns (resul_Value :type "Float (double-precision)"))
  (return (`KismetMathLibrary.FClamp` (+ (+ (+ (+ Base_Offset (* (`self.I/E`) Weight_E)) (* (`self.N/S`) Weight_N)) (* (`self.J/P`) Weight_T)) (* (`self.T/S`) Weight_J)) Min Max)))

(fn `CalculateDynamicSettigns`
  (returns (DynamicsSettings :type "/Game/TFG-Castellanos-Sanchez/Blueprints/Settings/ST_FacialSettings Structure"))
  (bind _resul_value (`self.Calculate_Single_CurveWithRange` 1.5 0.0 -0.5 -0.5 1.0 1.0 3.0))
  (bind _resul_value_2 (`self.Calculate_Single_CurveWithRange` -10.0 0.0 30.0 20.0 20.0 1.0 100.0))
  (bind _resul_value_3 (`self.Calculate_Single_CurveWithRange` 1.0 0.0 -0.3 -0.1 0.5 0.0 5.0))
  (bind _resul_value_4 (`self.Calculate_Single_CurveWithRange` 0.6 0.4 -0.2 -0.2 0.5 0.1 2.0))
  (return (make `/Game/TFG-Castellanos-Sanchez/Blueprints/Settings/ST_FacialSettings` _resul_value _resul_value_2 false 1.0 _resul_value_3 100.0 _resul_value_4 _resul_value _resul_value_2 false _resul_value_3 100.0 _resul_value_4 _resul_value _resul_value_2 true _resul_value_3 100.0 _resul_value_4 _resul_value _resul_value_2 _resul_value _resul_value_2 _resul_value _resul_value_2 true (`self.Calculate_Single_CurveWithRange` -1.5 -1.0 2.0 0.0 3.5 0.5 8.0) _resul_value _resul_value_2 true (`self.Calculate_Single_CurveWithRange` 1.0 0.0 -0.5 0.0 1.0 0.1 3.0) (`self.Calculate_Single_CurveWithRange` 1.0 0.0 0.0 -0.3 1.0 0.1 5.0) (`KismetMathLibrary.MakeVector2D` (`self.Calculate_Single_CurveWithRange` 15.0 10.0 0.0 -10.0 20.0 5.0 50.0) (`self.Calculate_Single_CurveWithRange` 7.5 5.0 0.0 -5.0 10.0 2.5 25.0)) (`KismetMathLibrary.MakeVector2D` (`self.Calculate_Single_CurveWithRange` 1.0 2.0 0.0 -0.5 1.0 0.2 5.0) (`self.Calculate_Single_CurveWithRange` 0.5 1.0 0.0 -0.25 0.5 0.1 2.5)))))

(fn `CalculateFaceTargets`
  (returns (Personality :type "/Game/TFG-Castellanos-Sanchez/Blueprints/Settings/ST_FacialPersonalitySettings Structure"))
  (return (make `/Game/TFG-Castellanos-Sanchez/Blueprints/Settings/ST_FacialPersonalitySettings` (`KismetMathLibrary.MakeVector2D` 0.0 (`self.Calculate_Single_Curve` -0.3 0.0 -0.2 0.1 0.1)) (`KismetMathLibrary.MakeVector2D` 0.0 (`self.Calculate_Single_Curve` 0.2 0.1 -0.1 -0.2 0.05)) 0.0 (`self.Calculate_Single_Curve` -0.2 0.4 0.1 -0.1) (`self.Calculate_Single_Curve` -0.2 0.1 0.7 0.3 -0.1) (`self.Calculate_Single_Curve` 0.3 0.6 -0.2 -0.1) (`KismetMathLibrary.MakeVector2D` 0.0 (`self.Calculate_Single_Curve` 0.0 0.3 -0.1 0.0 0.5)) (`self.Calculate_Single_Curve` 0.7 0.0 -0.1) (`KismetMathLibrary.MakeVector2D` 0.0 (`self.Calculate_Single_Curve` 0.1 0.0 0.2)) (`self.Calculate_Single_Curve` 0.0 0.0 0.3 0.1) (`self.Calculate_Single_Curve` 0.8 0.1 -0.2 -0.1) (`self.Calculate_Single_Curve` -0.5 0.0 0.2 0.4) (`self.Calculate_Single_Curve` -0.4 0.2) (`self.Calculate_Single_Curve` -0.3 0.0 0.1 0.1))))

(fn `CalculateRawCorporalTargets`
  (returns (Personality :type "/Game/TFG-Castellanos-Sanchez/Blueprints/Settings/ST_BodyPersonalitySettings Structure"))
  (return (make `/Game/TFG-Castellanos-Sanchez/Blueprints/Settings/ST_BodyPersonalitySettings` (`KismetMathLibrary.MakeRotator` 0.0 (`self.Calculate_Corporal_Canal` 0.22 -0.16 0.0 -0.06 0.5 0.0 8.0)) (`KismetMathLibrary.MakeRotator` 0.0 (`self.Calculate_Corporal_Canal` -0.25 0.2 0.03 0.08 0.35 -12.0 10.0)) (`KismetMathLibrary.MakeRotator` (`self.Calculate_Corporal_Canal` -0.03 0.18 0.04 0.05 0.35 0.0 7.0)) (`KismetMathLibrary.MakeRotator` 0.0 (`self.Calculate_Corporal_Canal` -0.06 0.2 0.02 0.06 0.38 -6.0 8.0)) (`KismetMathLibrary.MakeRotator` 0.0 (`self.Calculate_Corporal_Canal` -0.04 0.18 0.01 0.06 0.35 -8.0 10.0)) (`KismetMathLibrary.MakeRotator` 0.0 (`self.Calculate_Corporal_Canal` -0.04 0.08 0.18 0.2 0.4 0.8 1.5)))))

(fn `CorporalSettingsUpdate`
  (params (Target :type "Object Object Reference") (Time :type "Float (double-precision)"))
  (bind _transfer (`self.TransferCorporalSettigns` (`self.AuxCorporalPersonalitySettings`)))
  (bind _output_get (set `self.CorporalPersonalitySettings` _transfer))
  (message `/Game/TFG-Castellanos-Sanchez/Blueprints/ExpresionCorporal/BPI_BodyAnimation.Updater` Target _output_get (`self.Enabled`) (`self.IAEmotionsSettings`)))

(fn `Find Face`
  (params (Metahuman_in :type "Actor Object Reference"))
  ;[0 0.5833 0.07276 0.5] Find Face SkeletalMesh
  (`/Engine/EditorBlueprintResources/StandardMacros.IsValid` Metahuman_in
    (:`Is Valid`
      (if (not (`self.SetupCompleteExt`))
        (for _array_element (`self.K2_GetComponentsByClass` Metahuman_in "/Script/Engine.SkeletalMeshComponent")
          (if (`KismetStringLibrary.EqualEqual_StrStr` (`KismetSystemLibrary.GetObjectName` _array_element) (`self.HeadMeshName`))
            (bind _output_get (set `self.FaceMesh` _array_element))
            (bind _asanim_instance (castclass `AnimInstance` (`self.Animation_BP`)))
            (`SkeletalMeshComponent.SetOverridePostProcessAnimBP` _output_get _asanim_instance true)))
        (bind _facemesh (`self.FaceMesh`)
          (:`then`
            (bind _output_get_2 (set `self.InternalFaceAnimClass` (`SkeletalMeshComponent.GetPostProcessInstance` _facemesh)))
            (if (`KismetSystemLibrary.DoesImplementInterface` _output_get_2 "/Game/TFG-Castellanos-Sanchez/Blueprints/ExpresionesFaciales/BPI_FacialAnimation.BPI_FacialAnimation_C")
              (`self.SettingsUpdate` _output_get_2)
              ;;[0.6 0 0.04823] Run debug commands
              (if (`self.Debug`)
                (`KismetSystemLibrary.ExecuteConsoleCommand` "a.AnimNode.ControlRig.Debug 1" null)
                (`KismetSystemLibrary.ExecuteConsoleCommand` " ControlRig.EnableDrawInterfaceInGame 1" null))
              (set `self.SetupCompleteExt` true)))
          (:`else`))))))

(fn `Reset`
  ;[0.3906 0 0 0.5] Disable FacialAnim
  (set `self.IsTicking` false)
  (set `self.SetupCompleteExt` false))

(fn `SettingsUpdate`
  (params (TargetInst :type "Object Object Reference") (Time :type "Float (double-precision)"))
  (bind _personalitysettings (`self.SmoothingAll` (`self.AuxPerSettings`) Time))
  (bind (_personalitysettings_2 _settings) (`self.Transfer` _personalitysettings (`self.AuxDynSettings`)))
  (bind _output_get (set `self.FacialSettings` _settings))
  (bind _output_get_2 (set `self.FacialPersonalitySettings` _personalitysettings_2))
  (bind _curves (`self.Curves`)
    (:`then`
      (message `/Game/TFG-Castellanos-Sanchez/Blueprints/ExpresionesFaciales/BPI_FacialAnimation.Updater` TargetInst _output_get _curves (`self.Enabled`) _output_get_2 (`self.IAEmotionsSettings`)))
    (:`else`)))

(fn `SetupFacial`
  (bind _dynamicssettings (`self.CalculateDynamicSettigns`))
  (bind _output_get (set `self.AuxDynSettings` _dynamicssettings))
  (bind _personality (`self.CalculateFaceTargets`))
  (set `self.AuxPerSettings` _personality)
  (bind (_personalitysettings _settings) (`self.Transfer` _personality _output_get))
  (set `self.FacialSettings` _settings)
  (set `self.FacialPersonalitySettings` _personalitysettings))

(fn `Smoothing`
  (params (Current :type "Float (double-precision)") (Target :type "Float (double-precision)") (Time :type "Float (double-precision)"))
  (returns (Value :type "Float (double-precision)"))
  (return (`KismetMathLibrary.FInterpTo` Current Target Time (`self.Smoothing_Speed`))))

(fn `SmoothingAll`
  (params (Personality :type "/Game/TFG-Castellanos-Sanchez/Blueprints/Settings/ST_FacialPersonalitySettings Structure") (Time :type "Float (double-precision)"))
  (returns (PersonalitySettings :type "/Game/TFG-Castellanos-Sanchez/Blueprints/Settings/ST_FacialPersonalitySettings Structure"))
  (bind _facialpersonalitysettings (`self.FacialPersonalitySettings`))
  (if (> Time 0.0)
    (return (make `/Game/TFG-Castellanos-Sanchez/Blueprints/Settings/ST_FacialPersonalitySettings` (`KismetMathLibrary.MakeVector2D` 0.0 (`self.Smoothing` (`.Y` (`KismetMathLibrary.BreakVector2D` (break `/Game/TFG-Castellanos-Sanchez/Blueprints/Settings/ST_FacialPersonalitySettings` _facialpersonalitysettings))) (`.Y` (`KismetMathLibrary.BreakVector2D` Personality_C_Mouth_2_DDED24394C71C3F8568F86AF5A125521)) Time)) (`KismetMathLibrary.MakeVector2D` 0.0 (`self.Smoothing` (`.Y` (`KismetMathLibrary.BreakVector2D` (`.C_Jaw_4_3A4F5CC249A27FECA865C7ACCE1DC016` (break `/Game/TFG-Castellanos-Sanchez/Blueprints/Settings/ST_FacialPersonalitySettings` _facialpersonalitysettings)))) (`.Y` (`KismetMathLibrary.BreakVector2D` Personality_C_Jaw_4_3A4F5CC249A27FECA865C7ACCE1DC016)) Time)) (`self.Smoothing` (`.Blink_Eye_9_997579FC4612AA18A9AC1B92D4DDC3FB` (break `/Game/TFG-Castellanos-Sanchez/Blueprints/Settings/ST_FacialPersonalitySettings` _facialpersonalitysettings)) Personality_Blink_Eye_9_997579FC4612AA18A9AC1B92D4DDC3FB Time) (`self.Smoothing` (`.Brow_Lateral_11_D14B7A3A4703FB08A949B2A7D5AC7A21` (break `/Game/TFG-Castellanos-Sanchez/Blueprints/Settings/ST_FacialPersonalitySettings` _facialpersonalitysettings)) Personality_Brow_Lateral_11_D14B7A3A4703FB08A949B2A7D5AC7A21 Time) (`self.Smoothing` (`.Brow_Down_13_13E83A1744D5803A5F8E239057A2F38F` (break `/Game/TFG-Castellanos-Sanchez/Blueprints/Settings/ST_FacialPersonalitySettings` _facialpersonalitysettings)) Personality_Brow_Down_13_13E83A1744D5803A5F8E239057A2F38F Time) (`self.Smoothing` (`.Brow_Raise_15_14A59D9C44DB0F26D0A3B4B931BBFB71` (break `/Game/TFG-Castellanos-Sanchez/Blueprints/Settings/ST_FacialPersonalitySettings` _facialpersonalitysettings)) Personality_Brow_Raise_15_14A59D9C44DB0F26D0A3B4B931BBFB71 Time) (`KismetMathLibrary.MakeVector2D` 0.0 (`self.Smoothing` (`.Y` (`KismetMathLibrary.BreakVector2D` (`.C_Eye_34_C446514344708E891DC7DCA933DD895D` (break `/Game/TFG-Castellanos-Sanchez/Blueprints/Settings/ST_FacialPersonalitySettings` _facialpersonalitysettings)))) (`.Y` (`KismetMathLibrary.BreakVector2D` Personality_C_Eye_34_C446514344708E891DC7DCA933DD895D)) Time)) (`self.Smoothing` (`.Cheek_Raise_19_8A4168E142EA50BCC70C4E9D25FFEC12` (break `/Game/TFG-Castellanos-Sanchez/Blueprints/Settings/ST_FacialPersonalitySettings` _facialpersonalitysettings)) Personality_Cheek_Raise_19_8A4168E142EA50BCC70C4E9D25FFEC12 Time) (`KismetMathLibrary.MakeVector2D` 0.0 (`self.Smoothing` (`.Y` (`KismetMathLibrary.BreakVector2D` (`.L_R_Nose_22_84A0D89D4DCE84180C34009940E174C0` (break `/Game/TFG-Castellanos-Sanchez/Blueprints/Settings/ST_FacialPersonalitySettings` _facialpersonalitysettings)))) (`.Y` (`KismetMathLibrary.BreakVector2D` Personality_L_R_Nose_22_84A0D89D4DCE84180C34009940E174C0)) Time)) (`self.Smoothing` (`.Mouth_Upper_25_5DF8A302436C9962E7961A9A6F3EE18D` (break `/Game/TFG-Castellanos-Sanchez/Blueprints/Settings/ST_FacialPersonalitySettings` _facialpersonalitysettings)) Personality_Mouth_Upper_25_5DF8A302436C9962E7961A9A6F3EE18D Time) (`self.Smoothing` (`.Mouth_Corner_Pull_27_D77451D54FED636DE4C88A95079D7315` (break `/Game/TFG-Castellanos-Sanchez/Blueprints/Settings/ST_FacialPersonalitySettings` _facialpersonalitysettings)) Personality_Mouth_Corner_Pull_27_D77451D54FED636DE4C88A95079D7315 Time) (`self.Smoothing` (`.Mouth_Corner_Depress_29_415061F44EDA88E29F09569B53A15ECD` (break `/Game/TFG-Castellanos-Sanchez/Blueprints/Settings/ST_FacialPersonalitySettings` _facialpersonalitysettings)) Personality_Mouth_Corner_Depress_29_415061F44EDA88E29F09569B53A15ECD Time) (`self.Smoothing` (`.C_Neck_31_B4D4F14E4362C6BD7E831A9318B2E76B` (break `/Game/TFG-Castellanos-Sanchez/Blueprints/Settings/ST_FacialPersonalitySettings` _facialpersonalitysettings)) Personality_C_Neck_31_B4D4F14E4362C6BD7E831A9318B2E76B Time) (`self.Smoothing` (`.Mouth_Sticky_33_39C9853049B86400E000E2BB6C8DE3CB` (break `/Game/TFG-Castellanos-Sanchez/Blueprints/Settings/ST_FacialPersonalitySettings` _facialpersonalitysettings)) Personality_Mouth_Sticky_33_39C9853049B86400E000E2BB6C8DE3CB Time)))))

(fn `Transfer`
  (params (Personality :type "/Game/TFG-Castellanos-Sanchez/Blueprints/Settings/ST_FacialPersonalitySettings Structure") (Dynamics :type "/Game/TFG-Castellanos-Sanchez/Blueprints/Settings/ST_FacialSettings Structure"))
  (returns (PersonalitySettings :type "/Game/TFG-Castellanos-Sanchez/Blueprints/Settings/ST_FacialPersonalitySettings Structure") (Settings :type "/Game/TFG-Castellanos-Sanchez/Blueprints/Settings/ST_FacialSettings Structure"))
  (return (make `/Game/TFG-Castellanos-Sanchez/Blueprints/Settings/ST_FacialPersonalitySettings` Personality_C_Mouth_2_DDED24394C71C3F8568F86AF5A125521 Personality_C_Jaw_4_3A4F5CC249A27FECA865C7ACCE1DC016 Personality_Blink_Eye_9_997579FC4612AA18A9AC1B92D4DDC3FB Personality_Brow_Lateral_11_D14B7A3A4703FB08A949B2A7D5AC7A21 Personality_Brow_Down_13_13E83A1744D5803A5F8E239057A2F38F Personality_Brow_Raise_15_14A59D9C44DB0F26D0A3B4B931BBFB71 Personality_C_Eye_34_C446514344708E891DC7DCA933DD895D Personality_Cheek_Raise_19_8A4168E142EA50BCC70C4E9D25FFEC12 Personality_L_R_Nose_22_84A0D89D4DCE84180C34009940E174C0 Personality_Mouth_Upper_25_5DF8A302436C9962E7961A9A6F3EE18D Personality_Mouth_Corner_Pull_27_D77451D54FED636DE4C88A95079D7315 Personality_Mouth_Corner_Depress_29_415061F44EDA88E29F09569B53A15ECD Personality_C_Neck_31_B4D4F14E4362C6BD7E831A9318B2E76B Personality_Mouth_Sticky_33_39C9853049B86400E000E2BB6C8DE3CB) (make `/Game/TFG-Castellanos-Sanchez/Blueprints/Settings/ST_FacialSettings` Dynamics_Brows_3_F17CD7EA41C466B085AB05BCCCF85204 Dynamics_BrowsSmoothing_17_731916A944B3B885759EE681F168A4B0 Dynamics_BrowsUseDynamics_18_1B364FF344063B8E935E32B4B1F4BE90 Dynamics_Settings_Global_Control_111_24B8EDCC4A55E2825F41E1A7F0E66DB9 Dynamics_BrowsWiggleStrength_75_9A9D3F694D48F6BCB1941D8C507915E8 Dynamics_BrowsWiggleSmoothing_76_A61B39B142D3F210A1F089A5A0C9350F Dynamics_BrowsWiggleFrequency_77_A0A7C94A4E579F08980DA0875B801DA6 Dynamics_Nose_78_05AB4D9B4F4E23DD05A512B17268298D Dynamics_NoseSmoothing_79_74FE89D64325037EA1DB8C8BA011A8F2 Dynamics_NoseUseDynamics_28_C7C11401405A1C047E32AB80C42A79E3 Dynamics_NoseWiggleStrength_80_3889775344CDF3D77357CFB1C6759573 Dynamics_NoseWiggleSmoothing_81_2032E0B94B081F05880796961D9C7437 Dynamics_NoseWiggleFrequency_82_A4E18F31494B00A1074999A1DC91968F Dynamics_Cheeks_83_6A3F2E5343B1CFEB49DDB28F1A9581DD Dynamics_CheeksSmoothing_85_B32D532B40FD35C71819E68D0AE7F574 Dynamics_CheeksUseDynamics_39_0CB6379B40504CB6550B38AE11546E1E Dynamics_CheeksWiggleStrength_86_22DDA2CF4D1DFA76A924D0B4E8E6B32C Dynamics_CheeksWiggleSmoothing_87_031A513E4B757E74BEE89FA8F87AD4F1 Dynamics_CheeksWiggleFrequency_88_1A253EDE4B3FA88B08A7E1A1E6722DFA Dynamics_Mouth_89_7B9E3F0A4A85A9A25FEC02ACA6A22FC3 Dynamics_MouthSmoothing_90_D497F23A4FCB39D99550D4BAB522DD32 Dynamics_Jaw_91_DFB9674047B757654B0F6CAB7E3705FC Dynamics_JawSmoothing_92_D9AF913A4477FB833D077A96527E8C60 Dynamics_Eyes_93_31E1D0F6498EDA078B5390868C62D88C Dynamics_EyesSmoothing_94_DFEC0A9D4C40A004774C978D61D3491C Dynamics_GenerateBlinks_60_D2A11C1D42C86605DDED79948B2CC5BE Dynamics_BlinkInterval_95_F26C76CB4F926118BED3ED901B438242 Dynamics_Blinks_96_8C2075774F605B503BA535AB99C0F171 Dynamics_BlinksSmoothing_97_59ECB8B44A129AFA8E720FAF9CA99B2E Dynamics_UseBreathing_67_3C100D914739B104F7835BA1669F8202 Dynamics_BreathStrength_98_766F5BC842DD0FA843CB6E8999F715F8 Dynamics_BreathSpeed_99_64D68E7242F83DF39E06C39D978BF211 Dynamics_MicroSaccadicWeight_108_467A34244B9F6B340D52DFACA5AD504D Dynamics_MicroSaccadicSpeed_109_BD3179F843EF96B6F04A448182D62F32 Dynamics_MicroSaccadicEnabled_110_DF1911784263F1FFA58D3E842A760E1B 1.0 "NewEnumerator0" (`self.UseEmotion`))))

(fn `TransferCorporalSettigns`
  (params (Personality :type "/Game/TFG-Castellanos-Sanchez/Blueprints/Settings/ST_BodyPersonalitySettings Structure"))
  (returns (Transfer :type "/Game/TFG-Castellanos-Sanchez/Blueprints/Settings/ST_BodyPersonalitySettings Structure"))
  (return (make `/Game/TFG-Castellanos-Sanchez/Blueprints/Settings/ST_BodyPersonalitySettings` Personality_UpperBodyOpen_47_33E312344CC7AAF029C5F78D52D7E313 Personality_LeanForward_48_28A580D148BA28CFAE8D878E09E5E477 Personality_ShoulderDrop_49_3ED3CB354B43A32A59696EAF4DA15A5B Personality_NeckPitch_50_6CEC8DE643DB9D46ABB45C9C7C638C97 Personality_HeadPitch_51_A5846AEB48232614D50C749013ADF2F3 Personality_Rigidity_54_4C42EDD641A3587BCD42158B66CD0E03 1.0 1.0 "NewEnumerator0" (`self.UseEmotion`))))

(fn `Update`
  (params (Time :type "Float (double-precision)"))
  ;[0.15 0 0.004088 0.5] Anim Updater
  (`self.FaceMesh`
    (:`then`
      (`self.InternalFaceAnimClass`
        (:`then`
          _)
        (:`else`
          (bind _facemesh (`self.FaceMesh`)
            (:`then`
              (set `self.InternalFaceAnimClass` (`SkeletalMeshComponent.GetPostProcessInstance` _facemesh))
              (bind _internalfaceanimclass (`self.InternalFaceAnimClass`)
                (:`then`
                  _)
                (:`else`)))
            (:`else`))))
      (if (`KismetSystemLibrary.DoesImplementInterface` (`self.InternalFaceAnimClass`) "/Game/TFG-Castellanos-Sanchez/Blueprints/ExpresionesFaciales/BPI_FacialAnimation.BPI_FacialAnimation_C")
        (`self.SettingsUpdate` _internalfaceanimclass Time)
        (set `self.IsUpdatingExt` false)))
    (:`else`)))

(fn `UpdateCorporal`
  (params (Time :type "Float (double-precision)"))
  (bind _metahumanactor (`self.MetahumanActor`)
    (:`then`
      (bind _returnvalue (`SkeletalMeshComponent.GetAnimInstance` (`self.GetComponentByClass` _metahumanactor "/Script/Engine.SkeletalMeshComponent")))
      (if (`KismetSystemLibrary.DoesImplementInterface` _returnvalue "/Game/TFG-Castellanos-Sanchez/Blueprints/ExpresionCorporal/BPI_BodyAnimation.BPI_BodyAnimation_C")
        (`self.CorporalSettingsUpdate` _returnvalue Time)))
    (:`else`)))

(fn `UpdateEmotionsStruct`
  (params (In_EmotionMap :type "Map of String to Float (double-precision)"))
  (bind _keys (`BlueprintMapLibrary.Map_Keys` In_EmotionMap))
  (for _array_element _keys
    (`self.Apply_Emotion_To_Struct` (`BlueprintMapLibrary.Map_Find` In_EmotionMap _array_element) _array_element)))

(fn `UserConstructionScript`)