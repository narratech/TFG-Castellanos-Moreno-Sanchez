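; DoorInteractable is a hinged door that swings open and closed, toggled by its Open/Close event.
; A timeline, with play rate derived from OpeningTime, lerps the Hinge yaw to GradosGiro and reverses to close.
; On finish it updates IsOpen and re-enables CanInteract if BeInteractable is set.
; Interact, BeginPlay, focus and overlap events are empty, leaving the icon-widget and interaction-trigger logic disconnected.
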(event `self.ReceiveBeginPlay`)

(event `/Game/TFG-Castellanos-Moreno-Sanchez/Blueprints/Interfaces/Interactable.Interact`
  (params (PlayerRef :type "/Game/TFG-Castellanos-Moreno-Sanchez/Blueprints/FirstPerson/BP_DemoShooterCharacter Object Reference")))

(event `Open / Close`
  (`TimelineComponent.SetPlayRate` (`self.Open/Close_TL`) (/ 1.0 (`self.Opening_Time`)))
  (if (not (`self.Is_Open`))
    (bind (_direction _pista_nueva_0) (`Timeline|Open/Close_TL` :!via `PlayFromStart` :!label _label)
      (:`Update`
        (`SceneComponent.K2_SetRelativeRotation` (`self.Hinge`) (`KismetMathLibrary.MakeRotator` 0.0 0.0 (`KismetMathLibrary.Lerp` 0.0 (`self.GradosGiro`) _pista_nueva_0)) false false))
      (:`Finished`
        (switch `ETimelineDirection` _direction
          (:`Forward`
            (set `self.Is_Open` true))
          (:`Backward`
            (set `self.Is_Open` false)))
        (if (`self.Be_Interactable`)
          (set `self.CanInteract` true))))
    (else
      (goto _label :!via `ReverseFromEnd`))))

(event `self.Interaction_Icon_Show_Collision.OnComponentBeginOverlap`
  (params (OverlappedComponent :type "PrimitiveComponent Object Reference") (OtherActor :type "Actor Object Reference") (OtherComp :type "PrimitiveComponent Object Reference") (OtherBodyIndex :type Integer) (bFromSweep :type Boolean) (SweepResult :type "HitResult Structure (by ref)")))

(event `self.Interaction_Icon_Show_Collision.OnComponentEndOverlap`
  (params (OverlappedComponent :type "PrimitiveComponent Object Reference") (OtherActor :type "Actor Object Reference") (OtherComp :type "PrimitiveComponent Object Reference") (OtherBodyIndex :type Integer)))

(event `/Game/TFG-Castellanos-Moreno-Sanchez/Blueprints/Interfaces/Interactable.Set_Focus`
  (params (Focus :type Boolean)))

(fn `BeginPlay_Get_Refs`
  (bind _asw_interaction_icon (cast `/Game/TFG-Castellanos-Moreno-Sanchez/Blueprints/HUD/W_Interaction_Icon` (`WidgetComponent.GetWidget` (`self.Interact_Icon`))))
  (set `self.Interact_Ico_Widget_ref` _asw_interaction_icon))

(fn `Get_Details`
  (returns (Result :type Boolean))
  (return (`self.CanInteract`)))

(fn `UserConstructionScript`)