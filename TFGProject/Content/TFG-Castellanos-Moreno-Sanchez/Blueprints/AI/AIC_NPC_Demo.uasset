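; AI controller for demo NPCs that runs their behavior through a StateTree component.
; On BeginPlay it delays StateTree start, waiting longer on a dedicated server so clients can connect first.
; Every tick it draws a debug cone along its eye view, and a separate Debug function draws the pawn's control-rotation arrow through a Visual Logger drawer.
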(event `self.ReceiveTick`
  (params (DeltaSeconds :type "Float (single-precision)"))
  (bind (_outlocation _outrotation) (`self.GetActorEyesViewPoint`))
  (`KismetSystemLibrary.DrawDebugConeInDegrees` _outlocation (`KismetMathLibrary.Conv_RotatorToVector` _outrotation) 1500.0 45.0 45.0 12 (struct :`R` 0.095187 :`G` 0.043185 :`B` 1.0 :`A` 1.0)))

(event `self.ReceiveBeginPlay`
  (if (`KismetSystemLibrary.IsDedicatedServer`)
    (`KismetSystemLibrary.Delay` 8.0) ; We need to wait for clients to be connected.
    (else
      (`KismetSystemLibrary.Delay` 2.0)))
  (`BrainComponent.StartLogic` (`self.StateTreeAI`)))

(fn `Debug`
  (bind _returnvalue (`self.K2_GetPawn`))
  (bind _returnvalue_2 (`self.K2_GetActorLocation` _returnvalue))
  (`DrawDebugLibrary.DrawDebugArrow` (`DrawDebugLibrary.MakeVisualLoggerDebugDrawer` "Draw Debug Library") _returnvalue_2 (+ _returnvalue_2 (* (`KismetMathLibrary.GetForwardVector` (`Pawn.GetControlRotation` _returnvalue)) 50.0)) (struct :`LineType` "Solid" :`Color` (struct :`R` 1.0 :`B` 1.0 :`A` 1.0) :`DashWidth` 2.5 :`DashSpacing` 1.0 :`DotSpacing` 1.0) true (struct :`ArrowHeadStartSize` 5.0 :`ArrowHeadStartType` "Simple" :`bArrowheadOnEnd` true :`ArrowHeadEndSize` 5.0 :`ArrowHeadEndType` "Simple")))

(fn `UserConstructionScript`)